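; Base projectile actor that flies at a configurable speed and gravity, optionally aimed at or homing on a bound target.
; The construction script configures ProjectileMovement, including homing on BindTarget's root component when a target is valid.
; BeginPlay makes the collision box ignore the owner while moving and points velocity at the target.
; A hit fires the OnProjectileImpact dispatcher, spawns the impact effect and sound, then destroys the actor.
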(event OnComponentHit(BoxCollision)
  (params (HitComponent :type Primitive%20Component%20Object%20Reference) (OtherActor :type Actor%20Object%20Reference) (OtherComp :type Primitive%20Component%20Object%20Reference) (NormalImpulse :type Vector :default "0, 0, 0") (Hit :type Hit%20Result%20Structure%20%28by%20ref%29))
  (bind _location (Collision|BreakHitResult Hit))
  ;[0.15 0.15 0.15 0.5] On Impact
  (Default|CallOnProjectileImpact OtherActor Hit)
  (Effects|SpawnEmitteratLocation (Variables|Effects|GetImpactEffect) _location)
  (Audio|PlaySoundatLocation (Variables|Effects|GetDestroySoundEffect) _location "0, 0, 0" 1.0 1.0 0.0 0 0 0 0)
  (Actor|DestroyActor))

(event Custom|RotateToTarget
  ;[0.15 0.15 0.15 0.5] Constructor Begin
  (Variables|/Script/Engine.MovementComponent|SetVelocity (Variables|Default|GetProjectileMovement) (* (Math|Vector|GetUnitDirection(Vector) (Transformation|GetActorLocation) (Transformation|GetActorLocation (Variables|Target|GetBindTarget))) (Variables|ProjectileSettings|GetSpeed))))

(event EventBeginPlay
  ;[0.15 0.15 0.15 0.5] Constructor Begin
  (Collision|IgnoreActorwhenMoving (Variables|Default|GetBoxCollision) (Components|GetOwner) true)
  (Variables|Target|GetBindTarget
    (:then
      (CallFunction|RotatetoTarget))
    (:else)))

(event Collision|EventActorBeginOverlap
  (params (OtherActor :type Actor%20Object%20Reference)))

(event EventTick
  (params (DeltaSeconds :type Float%20%28single-precision%29)))

(fn ConstructionScript
  (bind _projectilemovement (Variables|Default|GetProjectileMovement))
  ;[0.15 0.15 0.15 0.5] Constructor
  (Variables|/Script/Engine.ProjectileMovementComponent|SetInitialSpeed _projectilemovement (Variables|ProjectileSettings|GetSpeed))
  (Variables|/Script/Engine.ProjectileMovementComponent|SetMaxSpeed _projectilemovement (Variables|ProjectileSettings|GetSpeed))
  (Variables|/Script/Engine.ProjectileMovementComponent|SetProjectileGravityScale _projectilemovement (Variables|ProjectileSettings|GetGravity))
  (Variables|Target|GetBindTarget
    (:then
      (if true
        (Variables|/Script/Engine.ProjectileMovementComponent|SetbIsHomingProjectile _projectilemovement (Variables|Target|GetisHoming))
        (Variables|/Script/Engine.ProjectileMovementComponent|SetHomingTargetComponent _projectilemovement (Variables|/Script/Engine.Actor|GetRootComponent (Variables|Target|GetBindTarget)))))
    (:else)))